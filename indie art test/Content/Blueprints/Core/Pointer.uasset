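; Pointer actor that displays a material billboard for a power-up type: speed, double jump or double points.
; On BeginPlay it checks the three boolean flags in that priority order and makes only the first matching billboard visible.
; It has no other active logic, as Tick, overlap and the construction script are empty.
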(event `self.ReceiveBeginPlay`
  (if (`self.Speed`)
    (`SceneComponent.SetVisibility` (`self.MaterialBillboard5`) true false)
    (elif (`self.DoubeJump`)
      (`SceneComponent.SetVisibility` (`self.MaterialBillboard4`) true false)
      (elif (`self.DoublePoints`)
        (`SceneComponent.SetVisibility` (`self.MaterialBillboard`) true false)))))

(fn `UserConstructionScript`)