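; Spline_collectable is an actor that spawns a row of collectible actors along its spline when play begins.
; BeginPlay divides the spline length by CollectionNum minus one to get even spacing, with one point at each end.
; It stores the world-space location at each distance in PointArray, then spawns the Collectible class at every stored point.
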(event `self.ReceiveBeginPlay`
  (bind _collection_num (`self.Collection Num`))
  (set `self.Subdivlen` (/ (`SplineComponent.GetSplineLength` (`self.Spline`)) (- _collection_num 1)))
  (for _index (range _collection_num)
    (`KismetArrayLibrary.Array_Add` (`self.point_array`) (`SplineComponent.GetLocationAtDistanceAlongSpline` (`self.Spline`) (* (`self.Subdivlen`) _index) "World")))
  (for _array_element (`self.point_array`)
    (`|SpawnActorFromClass` "/Game/Blueprints/Game_Components/Collectible.Collectible_C" (`KismetMathLibrary.MakeTransform` _array_element) "Undefined" "OverrideRootScale" null null)))

(fn `UserConstructionScript`)